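; AC_EffectsManager is an effects component for Character_Base owners that spawns text pop-ups and particle effects.
; On BeginPlay it caches its owner as a Character_Base reference.
; One event spawns a Text_spawner actor with the given text and color at the character's TextSpawnLoc.
; The other plays a passed-in particle system at the character's SpawnParticleEffect location.
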(event Custom|Spawn%20Text%20Pop-up
  (params (pop%20up%20text :type Text) (Text%20Color :type Color%20Structure))
  (Game|SpawnActorfromClass "/Game/RPG_System/Pop_Ups/Text_spawner.Text_spawner_C" (Math|Transform|MakeTransform (.Location (Math|Transform|BreakTransform (Transformation|GetWorldTransform (Variables|/Game/RPG_System/Character_Base.Character_Base_C|Gettext_Spawn_loc (Variables|Default|GetCharacterRef))))) "0,180.000000,0.000000") "Undefined" 0 pop%20up%20text Text%20Color 0))

(event Custom|Spawn%20Particles
  (params (ParticleTemplate :type Niagara%20System%20Object%20Reference))
  (Niagara|SpawnSystematLocation ParticleTemplate (Transformation|GetWorldLocation (Variables|/Game/RPG_System/Character_Base.Character_Base_C|Getspawn_particle_effect (Variables|Default|GetCharacterRef)))))

(event EventBeginPlay
  (bind _ascharacter_base (Utilities|Casting|CastToCharacter_Base (Components|GetOwner)))
  (Variables|Default|SetCharacterRef _ascharacter_base))