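; Character stats component that stores a character's combat values and processes incoming damage in the RPG battle system.
; SetCharacterData fills the stats, and CurrentHPToGlobalHP copies current HP into MinHP.
; ReciveDamage runs War (non-enemies only) and Plague crown effects from the controller's battle manager, subtracts HP, applies Death, messages the owner of damage or death, then calls Hunger on every crown.
; BeginPlay re-caches the game instance on a looping delay.
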(event EventBeginPlay
  (bind _asmain_game_instance (Utilities|Casting|CastToMain_GameInstance (Game|GetGameInstance) :!label _label))
  (Variables|Default|Setgame%20instance%20ref _asmain_game_instance)
  (Utilities|FlowControl|Delay 0.2)
  (goto _label))

(fn ReciveDamage
  (params (Damage :type Float%20%28single-precision%29) (whorecived :type Character%20Base%20Object%20Reference))
  (LocalVariables|SetDamageStorange Damage)
  (Utilities|FlowControl|Sequence
    (:then_0
      ;[1 1 1] активируем войну (когда другие получают урон, мы получаем его тоже
      (bind _ascharacter_base (Utilities|Casting|CastToCharacter_Base (Components|GetOwner)))
      (if (not (Variables|/Game/RPG_System/Character_Base.Character_Base_C|GetEnemy? _ascharacter_base))
        (bind _asmain_controller (Utilities|Casting|CastToMain_Controller (Game|GetPlayerController 0)))
        (for _array_element (Variables|/Game/RPG_System/Managers/AC_BattleManager.AC_BattleManager_C|GetCrowns (Variables|/Game/RPG_System/Main_Controller.Main_Controller_C|GetAC_BattleManager _asmain_controller))
          (if (Utilities|Enum|Equal(Enum) (Variables|/Game/RPG_System/Thrones/Thrones_Base.Thrones_Base_C|GetTypeOfThrone _array_element) "NewEnumerator2")
            (Default|ImplementWar(Debuff) _array_element (LocalVariables|GetDamageStorange) _ascharacter_base)))))
    (:then_1
      (bind _asmain_controller_2 (Utilities|Casting|CastToMain_Controller (Game|GetPlayerController 0)))
      (for _array_element_2 (Variables|/Game/RPG_System/Managers/AC_BattleManager.AC_BattleManager_C|GetCrowns (Variables|/Game/RPG_System/Main_Controller.Main_Controller_C|GetAC_BattleManager _asmain_controller_2))
        (if (Utilities|Enum|Equal(Enum) (Variables|/Game/RPG_System/Thrones/Thrones_Base.Thrones_Base_C|GetTypeOfThrone _array_element_2) "NewEnumerator3")
          (Default|ImplementPlague(Buff) _array_element_2 whorecived))))
    (:then_2
      ;[1 1 1] уменьшаем здоровье
      (Variables|CharStats|SetCurrentHP (- (Variables|CharStats|GetCurrentHP) (LocalVariables|GetDamageStorange)))
      (bind _asmain_controller_3 (Utilities|Casting|CastToMain_Controller (Game|GetPlayerController 0)))
      (bind _array_element_3 (Utilities|Array|ForEachLoopwithBreak (Variables|/Game/RPG_System/Managers/AC_BattleManager.AC_BattleManager_C|GetCrowns (Variables|/Game/RPG_System/Main_Controller.Main_Controller_C|GetAC_BattleManager _asmain_controller_3)))
        (:LoopBody
          (if (Utilities|Enum|Equal(Enum) (Variables|/Game/RPG_System/Thrones/Thrones_Base.Thrones_Base_C|GetTypeOfThrone _array_element_3) "NewEnumerator1")
            (Default|ImplementDeath(Buff) _array_element_3)))
        (:Completed
          (if (<= (Variables|CharStats|GetCurrentHP) 0.0)
            (Class|IDamage|EventonDeath(Message) (Components|GetOwner))
            (else
              ;[1 1 1] наносим дамаг
              (Variables|Default|SetRecivedDamage%28to%20text%29 (LocalVariables|GetDamageStorange))
              (Class|IDamage|EventonTakeDamage(Message) (Components|GetOwner)))))))
    (:then_4
      ;[1 1 1] вызываем голод (поглощаем урон)
      (bind _asmain_controller_4 (Utilities|Casting|CastToMain_Controller (Game|GetPlayerController 0)))
      (bind _array_element_4 (Utilities|Array|ForEachLoopwithBreak (Variables|/Game/RPG_System/Managers/AC_BattleManager.AC_BattleManager_C|GetCrowns (Variables|/Game/RPG_System/Main_Controller.Main_Controller_C|GetAC_BattleManager _asmain_controller_4)))
        (:LoopBody
          (bind _ascharacter_base_2 (Utilities|Casting|CastToCharacter_Base (Components|GetOwner)))
          (Default|ImplementHunger(Buff) _array_element_4 (LocalVariables|GetDamageStorange) _ascharacter_base_2))))))

(fn SetCharacterData
  (params (CharacterStats :type Map%20of%20E_CharStats%20Enums%20to%20Float%20%28single-precision%29s :default "NewEnumerator0") (HardDisplayName :type Name) (CurrentHP :type Float%20%28single-precision%29) (CurrentPower :type Float%20%28single-precision%29) (CurrentDefence :type Float%20%28single-precision%29) (CurrentCriticalHit :type Float%20%28single-precision%29) (CurrentMissHit :type Float%20%28single-precision%29) (CurrentCoolDown :type Float%20%28single-precision%29))
  (Variables|CharStats|SetCharacterStats CharacterStats)
  (Variables|CharStats|SetHardDisplayName HardDisplayName)
  (Variables|CharStats|SetCurrentHP CurrentHP)
  (Variables|CharStats|SetCurrentPower CurrentPower)
  (Variables|CharStats|SetCurrentDefence CurrentDefence)
  (Variables|CharStats|SetCurrentCriticalHit CurrentCriticalHit)
  (Variables|CharStats|SetCurrentMissHit CurrentMissHit)
  (Variables|CharStats|SetCurrentCoolDown CurrentCoolDown))

(fn CurrentHPtoGlobalHP
  (Variables|Default|SetMinHP (Variables|CharStats|GetCurrentHP)))