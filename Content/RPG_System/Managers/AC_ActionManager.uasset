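; Action manager component for turn-based RPG battles that executes the chosen Attack, Special Move or Switch Places through AC_BattleManager.
; Attacks roll miss and crit per selected target, apply defence-reduced damage and tick down the cooldown that gates special moves.
; Switching swaps transforms and turn order with a non-enemy target, then updates Crown throne effects (Hunger, War, Plague, Death).
; BeginPlay re-caches the game instance, which holds the selected targets, on a repeating delay loop.
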(event Custom|ExecuteAction
  (params (ActionType :type E_ActionType%20Enum :default "NewEnumerator0"))
  (bind _returnvalue (Game|GetPlayerController 0))
  (bind _returnvalue_2 (Actor|GetComponentbyClass _returnvalue "/Game/RPG_System/Managers/AC_BattleManager.AC_BattleManager_C"))
  (bind _currentcharacter (Variables|/Game/RPG_System/Managers/AC_BattleManager.AC_BattleManager_C|GetCurrentCharacter _returnvalue_2))
  (bind _ac_characterstats (Variables|/Game/RPG_System/Character_Base.Character_Base_C|GetAC_CharacterStats _currentcharacter))
  (bind _ac_characterstats_2 (Variables|/Game/RPG_System/Character_Base.Character_Base_C|GetAC_CharacterStats _currentcharacter))
  (switch Utilities|FlowControl|Switch|SwitchonE_ActionType ActionType
    (:NewEnumerator1
      (Utilities|FlowControl|Sequence
        (:then_0
          (Default|NormalAttack(flipbook) _currentcharacter)
          (Default|NormalAttack(ExtraEffects) _currentcharacter))
        (:then_1
          (CallFunction|ActivateAttack)
          (Variables|/Game/RPG_System/Managers/AC_CharacterStats.AC_CharacterStats_C|SetCurrentCoolDown _ac_characterstats (- (Variables|/Game/RPG_System/Managers/AC_CharacterStats.AC_CharacterStats_C|GetCurrentCoolDown _ac_characterstats) 1.0))
          (Default|FinishSelectAction _returnvalue_2 :!label _label))))
    (:NewEnumerator3
      (if (<= (Variables|/Game/RPG_System/Managers/AC_CharacterStats.AC_CharacterStats_C|GetCurrentCoolDown _ac_characterstats_2) 0.0)
        (Utilities|FlowControl|Sequence
          (:then_0
            (Default|SpecialAttack(animation) _currentcharacter))
          (:then_1
            (Default|SpecialAttack(Function) _currentcharacter)
            (Variables|/Game/RPG_System/Managers/AC_CharacterStats.AC_CharacterStats_C|SetCurrentCoolDown _ac_characterstats_2 (.Value (Utilities|Map|Find (Variables|/Game/RPG_System/Managers/AC_CharacterStats.AC_CharacterStats_C|GetCharacterStats _ac_characterstats_2) "NewEnumerator6")))
            (goto _label)))))
    (:NewEnumerator4
      (CallFunction|ActivateSwitch)
      (if (not (Variables|/Game/RPG_System/Character_Base.Character_Base_C|Getalreadewenttarget _currentcharacter))
        (goto _label)))))

(event EventBeginPlay
  (bind _asmain_game_instance (Utilities|Casting|CastToMain_GameInstance (Game|GetGameInstance) :!label _label))
  (Variables|Default|Setgame%20instance%20ref _asmain_game_instance)
  (Utilities|FlowControl|Delay 0.2)
  (goto _label))

(fn ActivateAttack
  (bind _asmain_controller (Utilities|Casting|CastToMain_Controller (Game|GetPlayerController 0)))
  (for _array_element (Variables|/Game/RPG_System/Main_GameInstance.Main_GameInstance_C|GetSelectedCharacterToAction (Variables|Default|Getgame%20instance%20ref))
    (if (<= (Math|Random|RandomFloatinRange 0.0 1.0) (Variables|/Game/RPG_System/Managers/AC_CharacterStats.AC_CharacterStats_C|GetCurrentMissHit (Variables|/Game/RPG_System/Character_Base.Character_Base_C|GetAC_CharacterStats (select (Variables|/Game/RPG_System/Managers/AC_BattleManager.AC_BattleManager_C|GetEnemyTurn? (Variables|/Game/RPG_System/Main_Controller.Main_Controller_C|GetAC_BattleManager _asmain_controller)) (Variables|/Game/RPG_System/Managers/AC_BattleManager.AC_BattleManager_C|GetCurrentEnemy (Variables|/Game/RPG_System/Main_Controller.Main_Controller_C|GetAC_BattleManager _asmain_controller)) (Variables|/Game/RPG_System/Managers/AC_BattleManager.AC_BattleManager_C|GetCurrentCharacter (Variables|/Game/RPG_System/Main_Controller.Main_Controller_C|GetAC_BattleManager _asmain_controller))))))
      (Default|SpawnTextPop-up (Variables|/Game/RPG_System/Character_Base.Character_Base_C|GetAC_EffectsManager _array_element) "МИМО" "NewEnumerator4" true)
      (elif (<= (Math|Random|RandomFloatinRange 0.0 1.0) (Variables|/Game/RPG_System/Managers/AC_CharacterStats.AC_CharacterStats_C|GetCurrentCriticalHit (Variables|/Game/RPG_System/Character_Base.Character_Base_C|GetAC_CharacterStats (select (Variables|/Game/RPG_System/Managers/AC_BattleManager.AC_BattleManager_C|GetEnemyTurn? (Variables|/Game/RPG_System/Main_Controller.Main_Controller_C|GetAC_BattleManager _asmain_controller)) (Variables|/Game/RPG_System/Managers/AC_BattleManager.AC_BattleManager_C|GetCurrentEnemy (Variables|/Game/RPG_System/Main_Controller.Main_Controller_C|GetAC_BattleManager _asmain_controller)) (Variables|/Game/RPG_System/Managers/AC_BattleManager.AC_BattleManager_C|GetCurrentCharacter (Variables|/Game/RPG_System/Main_Controller.Main_Controller_C|GetAC_BattleManager _asmain_controller))))))
        (Default|ReciveDamage (Variables|/Game/RPG_System/Character_Base.Character_Base_C|GetAC_CharacterStats _array_element) (* (+ (Variables|/Game/RPG_System/Managers/AC_CharacterStats.AC_CharacterStats_C|GetCurrentPower (Variables|/Game/RPG_System/Character_Base.Character_Base_C|GetAC_CharacterStats (select (Variables|/Game/RPG_System/Managers/AC_BattleManager.AC_BattleManager_C|GetEnemyTurn? (Variables|/Game/RPG_System/Main_Controller.Main_Controller_C|GetAC_BattleManager _asmain_controller)) (Variables|/Game/RPG_System/Managers/AC_BattleManager.AC_BattleManager_C|GetCurrentEnemy (Variables|/Game/RPG_System/Main_Controller.Main_Controller_C|GetAC_BattleManager _asmain_controller)) (Variables|/Game/RPG_System/Managers/AC_BattleManager.AC_BattleManager_C|GetCurrentCharacter (Variables|/Game/RPG_System/Main_Controller.Main_Controller_C|GetAC_BattleManager _asmain_controller))))) (Math|Random|RandomFloatinRange 0.25 0.5)) (- 1.0 (Variables|/Game/RPG_System/Managers/AC_CharacterStats.AC_CharacterStats_C|GetCurrentDefence (Variables|/Game/RPG_System/Character_Base.Character_Base_C|GetAC_CharacterStats _array_element)))) _array_element)
        (Default|SpawnTextPop-up (Variables|/Game/RPG_System/Character_Base.Character_Base_C|GetAC_EffectsManager _array_element) "КРИТИЧЕСКИЙ УРОН" "NewEnumerator5" true)
        (else
          (Default|ReciveDamage (Variables|/Game/RPG_System/Character_Base.Character_Base_C|GetAC_CharacterStats _array_element) (* (Variables|/Game/RPG_System/Managers/AC_CharacterStats.AC_CharacterStats_C|GetCurrentPower (Variables|/Game/RPG_System/Character_Base.Character_Base_C|GetAC_CharacterStats (select (Variables|/Game/RPG_System/Managers/AC_BattleManager.AC_BattleManager_C|GetEnemyTurn? (Variables|/Game/RPG_System/Main_Controller.Main_Controller_C|GetAC_BattleManager _asmain_controller)) (Variables|/Game/RPG_System/Managers/AC_BattleManager.AC_BattleManager_C|GetCurrentEnemy (Variables|/Game/RPG_System/Main_Controller.Main_Controller_C|GetAC_BattleManager _asmain_controller)) (Variables|/Game/RPG_System/Managers/AC_BattleManager.AC_BattleManager_C|GetCurrentCharacter (Variables|/Game/RPG_System/Main_Controller.Main_Controller_C|GetAC_BattleManager _asmain_controller))))) (- 1.0 (Variables|/Game/RPG_System/Managers/AC_CharacterStats.AC_CharacterStats_C|GetCurrentDefence (Variables|/Game/RPG_System/Character_Base.Character_Base_C|GetAC_CharacterStats _array_element)))) _array_element))))))

(fn ActivateSwitch
  (bind _returnvalue (Game|GetPlayerController 0))
  (bind _game_instance_ref (Variables|Default|Getgame%20instance%20ref))
  (bind _returnvalue_2 (Actor|GetComponentbyClass _returnvalue "/Game/RPG_System/Managers/AC_BattleManager.AC_BattleManager_C"))
  (bind _selectedcharactertoaction (Variables|/Game/RPG_System/Main_GameInstance.Main_GameInstance_C|GetSelectedCharacterToAction _game_instance_ref))
  (bind _output (Utilities|Array|Get(acopy) _selectedcharactertoaction))
  (bind _currentcharacter (Variables|/Game/RPG_System/Managers/AC_BattleManager.AC_BattleManager_C|GetCurrentCharacter _returnvalue_2))
  (Default|RefreshReference _returnvalue_2)
  (Variables|Default|Setprev_char%28for%20war%29 _currentcharacter)
  (Utilities|Array|Add (Variables|Default|GetReserved%20char) _currentcharacter)
  (bind _output_get (Variables|Default|SetReservedTransform (Transformation|GetActorTransform _output)))
  (if (not (Variables|/Game/RPG_System/Character_Base.Character_Base_C|GetEnemy? _output))
    (if (Utilities|Array|ContainsItem (Variables|Default|GetReserved%20char) _output)
      (Variables|/Game/RPG_System/Character_Base.Character_Base_C|Setalreadewenttarget _currentcharacter true)
      (else
        (Transformation|SetActorTransform _output (Transformation|GetActorTransform _currentcharacter))
        (Transformation|SetActorTransform _currentcharacter _output_get)
        (bind _output_get_2 (Variables|Default|SetReservedTurn (Variables|/Game/RPG_System/Character_Base.Character_Base_C|GetTurn _output)))
        (Variables|/Game/RPG_System/Character_Base.Character_Base_C|SetTurn _output (Variables|/Game/RPG_System/Character_Base.Character_Base_C|GetTurn _currentcharacter))
        (Variables|/Game/RPG_System/Character_Base.Character_Base_C|SetTurn _currentcharacter _output_get_2)
        (Utilities|FlowControl|Sequence
          (:then_0
            (Default|RefreshReference _returnvalue_2))
          (:then_1
            ;[1 1 1] вызываем голод при смене (убираем здоровье)
            (for _array_element (Variables|/Game/RPG_System/Managers/AC_BattleManager.AC_BattleManager_C|GetCrowns _returnvalue_2)
              (if (Utilities|Enum|Equal(Enum) (Variables|/Game/RPG_System/Thrones/Thrones_Base.Thrones_Base_C|GetTypeOfThrone _array_element) "NewEnumerator0")
                ;;[1 1 1] возвращаем процент здоровья прошлому владельцу голода
                (Default|HungerRestoreDebuff _array_element _currentcharacter)
                (Default|ImplementHunger(Debuff) _array_element false))))
          (:then_2
            (for _array_element_2 (Variables|/Game/RPG_System/Managers/AC_BattleManager.AC_BattleManager_C|GetCrowns _returnvalue_2)
              (if (Utilities|Enum|Equal(Enum) (Variables|/Game/RPG_System/Thrones/Thrones_Base.Thrones_Base_C|GetTypeOfThrone _array_element_2) "NewEnumerator2")
                (Default|ImplementWar(Buff) _array_element_2)
                (elif (Utilities|Enum|Equal(Enum) (Variables|/Game/RPG_System/Thrones/Thrones_Base.Thrones_Base_C|GetTypeOfThrone _array_element_2) "NewEnumerator3")
                  (Default|ImplementPlague(Debuff) _array_element_2)
                  (elif (Utilities|Enum|Equal(Enum) (Variables|/Game/RPG_System/Thrones/Thrones_Base.Thrones_Base_C|GetTypeOfThrone _array_element_2) "NewEnumerator1")
                    (Default|DeathRestore _array_element_2 (Variables|Default|Getprev_char%28for%20war%29))
                    (Default|ImplementDeath(Debuff) _array_element_2)))))))))))