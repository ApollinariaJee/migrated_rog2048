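; Enemy manager component that drives enemy attack choice and targeting in RPG battles.
; It copies spawn-point target lists into each assigned enemy's stats, then picks one at random and triggers the action manager and normal attack.
; The special-attack branch, which restores the stored cooldown, is unreachable because its condition is fixed true, so every choice decrements cooldown and attacks normally.
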(event EventBeginPlay
  (bind _asmain_game_instance (Utilities|Casting|CastToMain_GameInstance (Game|GetGameInstance) :!label _label))
  (Variables|Default|SetGameInstanceRef _asmain_game_instance)
  (Utilities|FlowControl|Delay 0.2)
  (goto _label))

(fn EnemyChooseAttack
  (bind (_currentenemy _battle_manager) (Utilities|CurrentEnemy))
  (bind _ac_characterstats (Variables|/Game/RPG_System/Character_Base.Character_Base_C|GetAC_CharacterStats _currentenemy))
  (Utilities|FlowControl|Sequence
    (:then_0
      (Utilities|FlowControl|Gate true :!label _label
        (:Exit
          (Variables|Default|SetStorageColldown (Variables|/Game/RPG_System/Managers/AC_CharacterStats.AC_CharacterStats_C|GetCurrentCoolDown _ac_characterstats))
          (goto _label Close))))
    (:then_1
      (if true
        (Variables|/Game/RPG_System/Managers/AC_CharacterStats.AC_CharacterStats_C|SetCurrentCoolDown _ac_characterstats (- (Variables|/Game/RPG_System/Managers/AC_CharacterStats.AC_CharacterStats_C|GetCurrentCoolDown _ac_characterstats) 1.0))
        (CallFunction|EnemyChooseTarget)
        (else
          (Default|SelectTarget _battle_manager "NewEnumerator3")
          (Class|IAttack|SpecialAttack(Function)(Message) _battle_manager)
          (Variables|/Game/RPG_System/Managers/AC_CharacterStats.AC_CharacterStats_C|SetCurrentCoolDown _ac_characterstats (Variables|Default|GetStorageColldown)))))))

(fn EnemyChooseTarget
  (bind _currentenemy (Utilities|CurrentEnemy))
  (Utilities|IsValid _currentenemy
    (:Is%20Valid
      (Utilities|Array|Add (Variables|/Game/RPG_System/Main_GameInstance.Main_GameInstance_C|GetSelectedCharacterToAction (Variables|Default|GetGameInstanceRef)) (.OutItem (Utilities|Array|Random (Variables|/Game/RPG_System/Managers/AC_CharacterStats.AC_CharacterStats_C|GetTargetedCharacters (Variables|/Game/RPG_System/Character_Base.Character_Base_C|GetAC_CharacterStats _currentenemy)))))
      (Default|ActivateAttack (Actor|GetComponentbyClass (Components|GetOwner) "/Game/RPG_System/Managers/AC_ActionManager.AC_ActionManager_C"))
      (Default|NormalAttack _currentenemy))))

(fn RefreshEnemy'sCharVariable
  (bind _outactors (Actor|GetAllActorsOfClass "/Game/RPG_System/SpawnPoints/Enemy_SpawnPoint.Enemy_SpawnPoint_C"))
  (bind _array_element (Utilities|Array|ForEachLoopwithBreak _outactors)
    (:LoopBody
      (Utilities|IsValid (Variables|/Game/RPG_System/SpawnPoints/Enemy_SpawnPoint.Enemy_SpawnPoint_C|GetAssignedEnemy _array_element)
        (:Is%20Valid
          (for _array_element_2 (Variables|/Game/RPG_System/SpawnPoints/Enemy_SpawnPoint.Enemy_SpawnPoint_C|GetAI_TargetedCharactersBase _array_element)
            (Utilities|Array|Add (Variables|/Game/RPG_System/Managers/AC_CharacterStats.AC_CharacterStats_C|GetTargetedCharacters (Variables|/Game/RPG_System/Character_Base.Character_Base_C|GetAC_CharacterStats (Variables|/Game/RPG_System/SpawnPoints/Enemy_SpawnPoint.Enemy_SpawnPoint_C|GetAssignedEnemy _array_element))) (Variables|/Game/RPG_System/SpawnPoints/Character_SpawnPoint.Character_SpawnPoint_C|GetAssignedChar _array_element_2))))))))