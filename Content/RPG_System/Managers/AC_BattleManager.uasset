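; Battle manager component that runs turn-based RPG fights between the party and level enemies.
; It spawns both sides from GameInstance maps and DataTables at slot-indexed spawn points, adding thrones for party members.
; ChangeTurn steps through each side, showing player action widgets or triggering enemy AI, recursing to swap sides and expiring character buffs.
; Action selection derives target candidates from DataTable target types, passing group targets straight to the action manager.
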(event Custom|delay_change_enemy_turn
  (Utilities|FlowControl|Delay 2.0)
  (In-Battle|ChangeTurn))

(event EventBeginPlay
  ;[1 1 1] Update GI reference
  (bind _asmain_game_instance (Utilities|Casting|CastToMain_GameInstance (Game|GetGameInstance) :!label _label))
  (Variables|Default|SetGameInstanceRef _asmain_game_instance)
  (Utilities|FlowControl|Delay 0.2)
  (goto _label))

(fn SpawnCharacters
  (bind _gameinstanceref (Variables|Default|GetGameInstanceRef))
  (bind _party (Variables|/Game/RPG_System/Main_GameInstance.Main_GameInstance_C|GetParty _gameinstanceref))
  (bind _values (Utilities|Map|Values _party))
  (for (_array_element _array_index) _values
    (bind _returnvalue (Utilities|GetDataTableRow "/Game/RPG_System/DataTable/DT_Character.DT_Character" (.NameHardCoded (Utilities|Struct|BreakS_Party _array_element)))
      (:then
        (bind _keys (Utilities|Map|Keys _party))
        (bind _returnvalue_2 (Game|SpawnActorfromClass (.CharacterActorClass (Utilities|Struct|BreakS_Character _returnvalue)) (.TransformLOCAL1 (Pre-Battle|FindTransform false (Utilities|Array|Get(acopy) _keys _array_index))) "Undefined" 0 self false 0 (Utilities|Array|Get(acopy) _keys _array_index) 0 0 0))
        (bind _returnvalue_3 (Game|SpawnActorfromClass "/Game/RPG_System/Thrones/Thrones_Base.Thrones_Base_C" (.TransformLOCAL1 (Pre-Battle|FindTransform false (Utilities|Array|Get(acopy) _keys _array_index))) "Undefined" _returnvalue_2 (.TypeOfSlot (Pre-Battle|FindTransform false (Utilities|Array|Get(acopy) _keys _array_index))) 0))
        (Utilities|Array|Add (Variables|Default|GetCrowns) _returnvalue_3)
        (Transformation|AttachComponentToComponent (Variables|/Game/RPG_System/Thrones/Thrones_Base.Thrones_Base_C|GetCrown_Particle _returnvalue_3) (Variables|/Game/RPG_System/SpawnPoints/Character_SpawnPoint.Character_SpawnPoint_C|Getparticle_spot (.CharacterSpot (Pre-Battle|FindTransform false (Utilities|Array|Get(acopy) _keys _array_index)))) "None" "KeepRelative" "KeepRelative" "SnapToTarget" true)
        (Transformation|AttachComponentToComponent (Variables|/Game/RPG_System/Thrones/Thrones_Base.Thrones_Base_C|GetPaperSprite _returnvalue_3) (Variables|/Game/RPG_System/SpawnPoints/Character_SpawnPoint.Character_SpawnPoint_C|Getcrown_spot (.CharacterSpot (Pre-Battle|FindTransform false (Utilities|Array|Get(acopy) _keys _array_index)))) "None" "KeepRelative" "KeepRelative" "KeepRelative" true)
        (Default|ChangeColor _returnvalue_3)
        (Utilities|Map|Add (Variables|CharacterBaseRef|GetSpawnedCharRef) (Utilities|Array|Get(acopy) _keys _array_index) _returnvalue_2)
        (Default|SetCharacterData (Variables|/Game/RPG_System/Character_Base.Character_Base_C|GetAC_CharacterStats _returnvalue_2) (.CharacterStats (Utilities|Struct|BreakS_Character _returnvalue)) (.CharacterHardCodedName (Utilities|Struct|BreakS_Character _returnvalue)) (.Value (Utilities|Map|Find (.CharacterStats (Utilities|Struct|BreakS_Character _returnvalue)) "NewEnumerator1")) (.Value (Utilities|Map|Find (.CharacterStats (Utilities|Struct|BreakS_Character _returnvalue)) "NewEnumerator3")) (.Value (Utilities|Map|Find (.CharacterStats (Utilities|Struct|BreakS_Character _returnvalue)) "NewEnumerator2")) (.Value (Utilities|Map|Find (.CharacterStats (Utilities|Struct|BreakS_Character _returnvalue)) "NewEnumerator5")) (.Value (Utilities|Map|Find (.CharacterStats (Utilities|Struct|BreakS_Character _returnvalue)) "NewEnumerator4")) (.Value (Utilities|Map|Find (.CharacterStats (Utilities|Struct|BreakS_Character _returnvalue)) "NewEnumerator6")))
        (Variables|/Game/RPG_System/SpawnPoints/Character_SpawnPoint.Character_SpawnPoint_C|SetAssignedChar (.CharacterSpot (Pre-Battle|FindTransform false (Utilities|Array|Get(acopy) _keys _array_index))) _returnvalue_2)
        (for _array_element_2 (Variables|/Game/RPG_System/SpawnPoints/Character_SpawnPoint.Character_SpawnPoint_C|GetTargetedEnemyBase (.CharacterSpot (Pre-Battle|FindTransform false (Utilities|Array|Get(acopy) _keys _array_index))))
          (Utilities|Array|Add (Variables|/Game/RPG_System/Managers/AC_CharacterStats.AC_CharacterStats_C|GetTargetedCharacters (Variables|/Game/RPG_System/Character_Base.Character_Base_C|GetAC_CharacterStats _returnvalue_2)) (Variables|/Game/RPG_System/SpawnPoints/Enemy_SpawnPoint.Enemy_SpawnPoint_C|GetAssignedEnemy _array_element_2)))))))

(fn SpawnEnemies
  (bind _gameinstanceref (Variables|Default|GetGameInstanceRef))
  (bind _enemiesononelevel (Variables|/Game/RPG_System/Main_GameInstance.Main_GameInstance_C|GetEnemiesOnOneLevel _gameinstanceref))
  (bind _keys (Utilities|Map|Keys _enemiesononelevel))
  (for _array_element _keys
    (bind _returnvalue (Utilities|GetDataTableRow "/Game/RPG_System/DataTable/DT_Enemies.DT_Enemies" (.Value (Utilities|Map|Find _enemiesononelevel _array_element)))
      (:then
        (bind _returnvalue_2 (Game|SpawnActorfromClass (.EnemyActorClass (Utilities|Struct|BreakS_Enemy _returnvalue)) (.TransformLOCAL1 (Pre-Battle|FindTransform true _array_element)) "Undefined" 0 self true 0 _array_element 0 0 0))
        (Utilities|Map|Add (Variables|CharacterBaseRef|GetSpawnedEnemyRef) _array_element _returnvalue_2)
        (Variables|/Game/RPG_System/SpawnPoints/Enemy_SpawnPoint.Enemy_SpawnPoint_C|SetAssignedEnemy (.EnemySpot (Pre-Battle|FindTransform true _array_element)) _returnvalue_2)
        (Default|SetCharacterData (Variables|/Game/RPG_System/Character_Base.Character_Base_C|GetAC_CharacterStats _returnvalue_2) (.EnemyStats (Utilities|Struct|BreakS_Enemy _returnvalue)) (.EbenyHardCodedName (Utilities|Struct|BreakS_Enemy _returnvalue)) (.Value (Utilities|Map|Find (.EnemyStats (Utilities|Struct|BreakS_Enemy _returnvalue)) "NewEnumerator1")) (.Value (Utilities|Map|Find (.EnemyStats (Utilities|Struct|BreakS_Enemy _returnvalue)) "NewEnumerator3")) (.Value (Utilities|Map|Find (.EnemyStats (Utilities|Struct|BreakS_Enemy _returnvalue)) "NewEnumerator2")) (.Value (Utilities|Map|Find (.EnemyStats (Utilities|Struct|BreakS_Enemy _returnvalue)) "NewEnumerator5")) (.Value (Utilities|Map|Find (.EnemyStats (Utilities|Struct|BreakS_Enemy _returnvalue)) "NewEnumerator4")) (.Value (Utilities|Map|Find (.EnemyStats (Utilities|Struct|BreakS_Enemy _returnvalue)) "NewEnumerator6")))))))

(fn ChangeTurn
  (if (Variables|Default|GetEnemyTurn?)
    ;[1 1 1] enemy change turn
    (bind _index (Utilities|FlowControl|ForLoopwithBreak 0 3 :!label _label)
      (:LoopBody
        (if (== _index 3)
          (Utilities|Array|Clear (Variables|CharacterBaseRef|GetAlreadyUsedCharacters))
          (Variables|Default|Setnextturn 0)
          (Variables|CharacterBaseRef|SetCurrentEnemy 0)
          (Variables|Default|SetEnemyTurn? false)
          (In-Battle|ChangeTurn)
          (else
            (Utilities|IsValid (Variables|CharacterBaseRef|GetCurrentEnemy)
              (:Is%20Valid
                (Development|SetHiddeninGame (Variables|/Game/RPG_System/Character_Base.Character_Base_C|Gettarget_cude (Variables|CharacterBaseRef|GetCurrentEnemy)) true false))
              (:Is%20Not%20Valid
                _))
            (if (.ReturnValue (Utilities|Map|Find (Variables|CharacterBaseRef|GetSpawnedEnemyRef) (Variables|Default|Getnextturn)))
              (if (Utilities|Array|ContainsItem (Variables|CharacterBaseRef|GetAlreadyUsedCharacters) (.Value (Utilities|Map|Find (Variables|CharacterBaseRef|GetSpawnedEnemyRef) (Variables|Default|Getnextturn))))
                (Variables|Default|Setnextturn (+ (Variables|Default|Getnextturn) 1) :!label _label_2)
                (else
                  (bind _output_get (Variables|CharacterBaseRef|SetCurrentEnemy (.Value (Utilities|Map|Find (Variables|CharacterBaseRef|GetSpawnedEnemyRef) (Variables|Default|Getnextturn)))))
                  (Utilities|IsValid _output_get
                    (:Is%20Valid
                      (Development|SetHiddeninGame (Variables|/Game/RPG_System/Character_Base.Character_Base_C|Gettarget_cude _output_get) false false)
                      (Utilities|Array|Add (Variables|CharacterBaseRef|GetAlreadyUsedCharacters) _output_get)
                      (bind _asmain_controller (Utilities|Casting|CastToMain_Controller (Game|GetPlayerController 0)))
                      (Default|EnemyChooseAttack (Variables|/Game/RPG_System/Main_Controller.Main_Controller_C|GetAC_EnemyManager _asmain_controller))
                      (Utilities|FlowControl|Sequence
                        (:then_0
                          (if (Variables|Default|GetEnemyTurn?)
                            (CallFunction|DelayChangeEnemyTurn)))
                        (:then_1
                          (goto _label Break)))))))
              (else
                (goto _label_2)))))))
    (else
      (Utilities|FlowControl|Sequence
        (:then_0
          ;[1 1 1] character change turn
          (Utilities|IsValid (Variables|UI|GetActionWidget)
            (:Is%20Valid
              (Widget|RemovefromParent (Variables|UI|GetActionWidget)))
            (:Is%20Not%20Valid
              _))
          (bind _index_2 (Utilities|FlowControl|ForLoopwithBreak 0 3 :!label _label_3)
            (:LoopBody
              (if (== _index_2 3)
                (Utilities|Array|Clear (Variables|CharacterBaseRef|GetAlreadyUsedCharacters))
                (Variables|Default|Setnextturn 0)
                (Variables|CharacterBaseRef|SetCurrentCharacter 0)
                (Variables|Default|SetEnemyTurn? true)
                (Widget|RemovefromParent (Variables|UI|GetActionWidget))
                (In-Battle|ChangeTurn)
                (else
                  (Utilities|IsValid (Variables|CharacterBaseRef|GetCurrentCharacter)
                    (:Is%20Valid
                      (Development|SetHiddeninGame (Variables|/Game/RPG_System/Character_Base.Character_Base_C|Gettarget_cude (Variables|CharacterBaseRef|GetCurrentCharacter)) true false))
                    (:Is%20Not%20Valid
                      _))
                  (if (.ReturnValue (Utilities|Map|Find (Variables|CharacterBaseRef|GetSpawnedCharRef) (Variables|Default|Getnextturn)))
                    (if (Utilities|Array|ContainsItem (Variables|CharacterBaseRef|GetAlreadyUsedCharacters) (.Value (Utilities|Map|Find (Variables|CharacterBaseRef|GetSpawnedCharRef) (Variables|Default|Getnextturn))))
                      (Variables|Default|Setnextturn (+ (Variables|Default|Getnextturn) 1) :!label _label_4)
                      (else
                        (bind _output_get_2 (Variables|CharacterBaseRef|SetCurrentCharacter (.Value (Utilities|Map|Find (Variables|CharacterBaseRef|GetSpawnedCharRef) (Variables|Default|Getnextturn)))))
                        (Development|SetHiddeninGame (Variables|/Game/RPG_System/Character_Base.Character_Base_C|Gettarget_cude _output_get_2) false false)
                        (Utilities|Array|Add (Variables|CharacterBaseRef|GetAlreadyUsedCharacters) _output_get_2)
                        (bind _returnvalue (UserInterface|CreateWidget "/Game/RPG_System/UI/WBP_ActionWidget.WBP_ActionWidget_C" (Game|GetPlayerController 0)))
                        (UserInterface|Viewport|AddtoViewport _returnvalue 0)
                        (Variables|UI|SetActionWidget _returnvalue)
                        (Utilities|FlowControl|Sequence
                          (:then_0
                            (goto _label_3 Break))
                          (:then_1
                            (In-Battle|ActivateThrone)))))
                    (else
                      (goto _label_4))))))))
        (:then_1
          ;[1 1 1] считает сколько ходов действуют баффы и после окончания ресетает статы
          (Utilities|IsValid (Variables|CharacterBaseRef|GetCurrentCharacter)
            (:Is%20Valid
              (if (Variables|/Game/RPG_System/Managers/AC_CharacterStats.AC_CharacterStats_C|GetStartCountingTurns (Variables|/Game/RPG_System/Character_Base.Character_Base_C|GetAC_CharacterStats (Variables|CharacterBaseRef|GetCurrentCharacter)))
                (bind _output_get_3 (Variables|/Game/RPG_System/Managers/AC_CharacterStats.AC_CharacterStats_C|SetNumberOfTurns (Variables|/Game/RPG_System/Character_Base.Character_Base_C|GetAC_CharacterStats (Variables|CharacterBaseRef|GetCurrentCharacter)) (Math|Integer|Min(Integer) (+ (Variables|/Game/RPG_System/Managers/AC_CharacterStats.AC_CharacterStats_C|GetNumberOfTurns (Variables|/Game/RPG_System/Character_Base.Character_Base_C|GetAC_CharacterStats (Variables|CharacterBaseRef|GetCurrentCharacter))) 1) (Variables|/Game/RPG_System/Managers/AC_CharacterStats.AC_CharacterStats_C|GetMaxTurnsAllowed (Variables|/Game/RPG_System/Character_Base.Character_Base_C|GetAC_CharacterStats (Variables|CharacterBaseRef|GetCurrentCharacter))))))
                (if (== _output_get_3 (Variables|/Game/RPG_System/Managers/AC_CharacterStats.AC_CharacterStats_C|GetMaxTurnsAllowed (Variables|/Game/RPG_System/Character_Base.Character_Base_C|GetAC_CharacterStats (Variables|CharacterBaseRef|GetCurrentCharacter))))
                  (Variables|/Game/RPG_System/Managers/AC_CharacterStats.AC_CharacterStats_C|SetNumberOfTurns (Variables|/Game/RPG_System/Character_Base.Character_Base_C|GetAC_CharacterStats (Variables|CharacterBaseRef|GetCurrentCharacter)) 0)
                  (Default|SetCharacterData (Variables|/Game/RPG_System/Character_Base.Character_Base_C|GetAC_CharacterStats (Variables|CharacterBaseRef|GetCurrentCharacter)) (Variables|/Game/RPG_System/Managers/AC_CharacterStats.AC_CharacterStats_C|GetCharacterStats (Variables|/Game/RPG_System/Character_Base.Character_Base_C|GetAC_CharacterStats (Variables|CharacterBaseRef|GetCurrentCharacter))) "None" (.Value (Utilities|Map|Find (Variables|/Game/RPG_System/Managers/AC_CharacterStats.AC_CharacterStats_C|GetCharacterStats (Variables|/Game/RPG_System/Character_Base.Character_Base_C|GetAC_CharacterStats (Variables|CharacterBaseRef|GetCurrentCharacter))) "NewEnumerator1")) (.Value (Utilities|Map|Find (Variables|/Game/RPG_System/Managers/AC_CharacterStats.AC_CharacterStats_C|GetCharacterStats (Variables|/Game/RPG_System/Character_Base.Character_Base_C|GetAC_CharacterStats (Variables|CharacterBaseRef|GetCurrentCharacter))) "NewEnumerator3")) (.Value (Utilities|Map|Find (Variables|/Game/RPG_System/Managers/AC_CharacterStats.AC_CharacterStats_C|GetCharacterStats (Variables|/Game/RPG_System/Character_Base.Character_Base_C|GetAC_CharacterStats (Variables|CharacterBaseRef|GetCurrentCharacter))) "NewEnumerator2")) (.Value (Utilities|Map|Find (Variables|/Game/RPG_System/Managers/AC_CharacterStats.AC_CharacterStats_C|GetCharacterStats (Variables|/Game/RPG_System/Character_Base.Character_Base_C|GetAC_CharacterStats (Variables|CharacterBaseRef|GetCurrentCharacter))) "NewEnumerator5")) (.Value (Utilities|Map|Find (Variables|/Game/RPG_System/Managers/AC_CharacterStats.AC_CharacterStats_C|GetCharacterStats (Variables|/Game/RPG_System/Character_Base.Character_Base_C|GetAC_CharacterStats (Variables|CharacterBaseRef|GetCurrentCharacter))) "NewEnumerator4")) 0.0))))))))))

(fn FindTransform
  (params (IsEnemy? :type Boolean) (Turn :type Integer))
  (if IsEnemy?
    (bind _outactors (Actor|GetAllActorsOfClass "/Game/RPG_System/SpawnPoints/Enemy_SpawnPoint.Enemy_SpawnPoint_C"))
    (bind _array_element (Utilities|Array|ForEachLoopwithBreak _outactors :!label _label)
      (:LoopBody
        (if (== (Variables|/Game/RPG_System/SpawnPoints/Enemy_SpawnPoint.Enemy_SpawnPoint_C|Getslotindex _array_element) Turn)
          (LocalVariables|SetTransformLOCAL (Math|Transform|MakeTransform (Transformation|GetActorLocation _array_element) (.rotation (Transformation|GetWorldTransform (Variables|/Game/RPG_System/SpawnPoints/Enemy_SpawnPoint.Enemy_SpawnPoint_C|GetArrow _array_element))) (.scale (Transformation|GetWorldTransform (Variables|/Game/RPG_System/SpawnPoints/Enemy_SpawnPoint.Enemy_SpawnPoint_C|GetArrow _array_element)))))
          (goto _label Break)))
      (:Completed
        (return (LocalVariables|GetTransformLOCAL) _array_element 0 "NewEnumerator0")))
    (else
      (bind _outactors_2 (Actor|GetAllActorsOfClass "/Game/RPG_System/SpawnPoints/Character_SpawnPoint.Character_SpawnPoint_C"))
      (bind _array_element_2 (Utilities|Array|ForEachLoopwithBreak _outactors_2 :!label _label_2)
        (:LoopBody
          (if (== (Variables|/Game/RPG_System/SpawnPoints/Character_SpawnPoint.Character_SpawnPoint_C|Getslotindex _array_element_2) Turn)
            (LocalVariables|SetTransformLOCAL (Math|Transform|MakeTransform (Transformation|GetActorLocation _array_element_2) (.rotation (Transformation|GetWorldTransform (Variables|/Game/RPG_System/SpawnPoints/Character_SpawnPoint.Character_SpawnPoint_C|GetArrow _array_element_2))) (.scale (Transformation|GetWorldTransform (Variables|/Game/RPG_System/SpawnPoints/Character_SpawnPoint.Character_SpawnPoint_C|GetArrow _array_element_2)))))
            (goto _label_2 Break)))
        (:Completed
          (return (LocalVariables|GetTransformLOCAL) 0 _array_element_2 (Variables|/Game/RPG_System/SpawnPoints/Character_SpawnPoint.Character_SpawnPoint_C|GetTypeOfSlot _array_element_2)))))))

(fn RefreshReference
  (bind _values (Utilities|Map|Values (Variables|CharacterBaseRef|GetSpawnedCharRef)))
  (for _array_element _values
    (Utilities|Map|Add (Variables|CharacterBaseRef|GetSpawnedCharRef) (Variables|/Game/RPG_System/Character_Base.Character_Base_C|GetTurn _array_element) _array_element)))

(fn SelectAction
  (params (ActionType :type E_ActionType%20Enum :default "NewEnumerator0"))
  (bind _selectui (Variables|UI|GetSelectUI))
  (Utilities|IsValid _selectui
    (:Is%20Valid
      (Widget|RemovefromParent _selectui))
    (:Is%20Not%20Valid
      _))
  (bind _output_get (Variables|/Game/RPG_System/Managers/AC_CharacterStats.AC_CharacterStats_C|SetSelectedActionType (Variables|/Game/RPG_System/Character_Base.Character_Base_C|GetAC_CharacterStats (Variables|CharacterBaseRef|GetCurrentCharacter)) ActionType))
  (Variables|Default|Setactivated true)
  (switch Utilities|FlowControl|Switch|SwitchonE_ActionType _output_get
    (:NewEnumerator1
      _)
    (:NewEnumerator3
      _)
    (:NewEnumerator4
      _))
  (In-Battle|SelectTarget _output_get))

(fn SelectTarget
  (params (ActionType :type E_ActionType%20Enum :default "NewEnumerator0"))
  (bind _enemyturn_ (Variables|Default|GetEnemyTurn?))
  (bind _returnvalue (UserInterface|CreateWidget "/Game/RPG_System/UI/WBP_ChooseDebug.WBP_ChooseDebug_C" (Game|GetPlayerController 0) ActionType))
  (Variables|UI|SetSelectUI _returnvalue)
  (UserInterface|Viewport|AddtoViewport _returnvalue 0)
  (if _enemyturn_
    (bind _returnvalue_2 (Utilities|GetDataTableRow "/Game/RPG_System/DataTable/DT_Character.DT_Character" (Variables|/Game/RPG_System/Managers/AC_CharacterStats.AC_CharacterStats_C|GetHardDisplayName (Variables|/Game/RPG_System/Character_Base.Character_Base_C|GetAC_CharacterStats (Variables|CharacterBaseRef|GetCurrentEnemy))))
      (:then
        _))
    (else
      (bind _returnvalue_3 (Utilities|GetDataTableRow "/Game/RPG_System/DataTable/DT_Character.DT_Character" (Variables|/Game/RPG_System/Managers/AC_CharacterStats.AC_CharacterStats_C|GetHardDisplayName (Variables|/Game/RPG_System/Character_Base.Character_Base_C|GetAC_CharacterStats (Variables|CharacterBaseRef|GetCurrentCharacter))))
        (:then
          _))))
  (switch Utilities|FlowControl|Switch|SwitchonE_ActionType ActionType
    (:NewEnumerator1
      (Variables|Default|Settargettype (select _enemyturn_ (.TargetsRegularAttack (Utilities|Struct|BreakS_Character _returnvalue_2)) (.TargetsRegularAttack (Utilities|Struct|BreakS_Character _returnvalue_3)))))
    (:NewEnumerator3
      (Variables|Default|Settargettype (select _enemyturn_ (.TargetsSpecialAttack (Utilities|Struct|BreakS_Character _returnvalue_2)) (.TargetsSpecialAttack (Utilities|Struct|BreakS_Character _returnvalue_3)))))
    (:NewEnumerator4
      (Variables|Default|Settargettype "NewEnumerator2")))
  (Utilities|Array|Clear (Variables|CharacterBaseRef|GetTargetedCharNow))
  (In-Battle|FillSelectedCharFer ActionType))

(fn FinishSelectAction
  (Widget|RemovefromParent (Variables|UI|GetSelectUI))
  (In-Battle|ChangeTurn)
  (Utilities|Array|Clear (Variables|/Game/RPG_System/Main_GameInstance.Main_GameInstance_C|GetSelectedCharacterToAction (Variables|Default|GetGameInstanceRef))))

(fn FillSelectedCharFer
  (params (ActionType :type E_ActionType%20Enum :default "NewEnumerator0"))
  (switch Utilities|FlowControl|Switch|SwitchonE_TargetingType (Variables|Default|Gettargettype)
    (:NewEnumerator0
      (Utilities|Array|Add (Variables|CharacterBaseRef|GetTargetedCharNow) (select (Variables|Default|GetEnemyTurn?) (Variables|CharacterBaseRef|GetCurrentEnemy) (Variables|CharacterBaseRef|GetCurrentCharacter))))
    (:NewEnumerator2
      (bind _values (Utilities|Map|Values (Variables|CharacterBaseRef|GetSpawnedCharRef)))
      (for _array_element _values
        (Utilities|Array|Add (Variables|CharacterBaseRef|GetTargetedCharNow) _array_element)))
    (:NewEnumerator3
      (bind _values_2 (Utilities|Map|Values (Variables|CharacterBaseRef|GetSpawnedCharRef)))
      (for _array_element_2 _values_2
        (Utilities|Array|Add (Variables|/Game/RPG_System/Main_GameInstance.Main_GameInstance_C|GetSelectedCharacterToAction (Variables|Default|GetGameInstanceRef)) _array_element_2))
      (bind _asmain_controller (Utilities|Casting|CastToMain_Controller (Game|GetPlayerController 0) :!label _label))
      (Default|SelectAction (Variables|/Game/RPG_System/Main_Controller.Main_Controller_C|GetAC_ActionManager _asmain_controller) ActionType))
    (:NewEnumerator4
      (bind _values_3 (Utilities|Map|Values (Variables|CharacterBaseRef|GetSpawnedEnemyRef)))
      (for _array_element_3 _values_3
        (Utilities|Array|Add (Variables|/Game/RPG_System/Main_GameInstance.Main_GameInstance_C|GetSelectedCharacterToAction (Variables|Default|GetGameInstanceRef)) _array_element_3))
      (goto _label))
    (:NewEnumerator5
      (bind _values_4 (Utilities|Map|Values (Variables|CharacterBaseRef|GetSpawnedEnemyRef)))
      (for _array_element_4 _values_4
        (Utilities|Array|Add (Variables|CharacterBaseRef|GetTargetedCharNow) _array_element_4)))
    (:NewEnumerator6
      (for _array_element_5 (Variables|/Game/RPG_System/Managers/AC_CharacterStats.AC_CharacterStats_C|GetTargetedCharacters (Variables|/Game/RPG_System/Character_Base.Character_Base_C|GetAC_CharacterStats (Variables|CharacterBaseRef|GetCurrentCharacter)))
        (Utilities|Array|Add (Variables|CharacterBaseRef|GetTargetedCharNow) _array_element_5)))
    (:NewEnumerator7
      (bind _values_5 (Utilities|Map|Values (Variables|CharacterBaseRef|GetSpawnedEnemyRef)))
      (for _array_element_6 _values_5
        (Utilities|Array|Add (Variables|/Game/RPG_System/Main_GameInstance.Main_GameInstance_C|GetSelectedCharacterToAction (Variables|Default|GetGameInstanceRef)) _array_element_6))
      (bind _values_6 (Utilities|Map|Values (Variables|CharacterBaseRef|GetSpawnedCharRef)))
      (for _array_element_7 _values_6
        (Utilities|Array|Add (Variables|/Game/RPG_System/Main_GameInstance.Main_GameInstance_C|GetSelectedCharacterToAction (Variables|Default|GetGameInstanceRef)) _array_element_7))
      (goto _label))
    (:NewEnumerator8
      (bind _values_7 (Utilities|Map|Values (Variables|CharacterBaseRef|GetSpawnedEnemyRef)))
      (for _array_element_8 _values_7
        (Utilities|Array|Add (Variables|CharacterBaseRef|GetTargetedCharNow) _array_element_8)))
    (:NewEnumerator9
      (bind _values_8 (Utilities|Map|Values (Variables|CharacterBaseRef|GetSpawnedCharRef)))
      (for _array_element_9 _values_8
        (Utilities|Array|Add (Variables|CharacterBaseRef|GetTargetedCharNow) _array_element_9)))))

(fn ActivateThrone
  (bind _outactors (Actor|GetAllActorsOfClass "/Game/RPG_System/SpawnPoints/Character_SpawnPoint.Character_SpawnPoint_C"))
  (for _array_element _outactors
    (Utilities|IsValid (Variables|/Game/RPG_System/SpawnPoints/Character_SpawnPoint.Character_SpawnPoint_C|GetAssignedChar _array_element)
      (:Is%20Valid
        (switch int (Variables|/Game/RPG_System/Character_Base.Character_Base_C|GetTurn (Variables|/Game/RPG_System/SpawnPoints/Character_SpawnPoint.Character_SpawnPoint_C|GetAssignedChar _array_element)))))))